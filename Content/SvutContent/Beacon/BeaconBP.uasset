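; Beacon lift that shuttles between three floor markers, starting at Floor2 and setting off when the first-person character overlaps the actor.
; A Move timeline lerps the lift mesh with sweep, then plays a camera shake on arrival if the player is aboard.
; IAmSoSorry selects the next stop in ping-pong order using GoingUp.
; CheckIfPlayerDown sends the lift down from Floor3 when the player is below BeaconHeight.
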(event `self.ReceiveBeginPlay`
  (bind _previousfloor_location (`KismetMathLibrary.BreakTransform` (`self.PreviousFloor`)))
  (set `self.PreviousFloor` (`SceneComponent.GetRelativeTransform` (`self.Floor 2`)))
  (set `self.Destination` (`SceneComponent.GetRelativeTransform` (`self.Floor 3`)))
  (`SceneComponent.K2_SetRelativeLocation` (`self.Beacon_ver_2_Lift_detail_1`) _previousfloor_location true false))

(event `self.ReceiveActorEndOverlap`
  (params (OtherActor :type "Actor Object Reference"))
  (cast `/Game/FirstPerson/Blueprints/BP_FirstPersonCharacter` OtherActor)
  (set `self.isPlayerAboard?` false)
  (if (not (`self.moves`))
    (`KismetSystemLibrary.Delay` 0.2)
    (`self.CheckIfPlayerDown`)))

(event `self.ReceiveActorBeginOverlap`
  (params (OtherActor :type "Actor Object Reference"))
  (bind _asbp_first_person_character (cast `/Game/FirstPerson/Blueprints/BP_FirstPersonCharacter` OtherActor))
  (set `self.Player` _asbp_first_person_character)
  (set `self.isPlayerAboard?` true)
  (if (not (`self.moves`))
    (`self.Lift`)))

(event `Lift`
  (bind _previousfloor_location (`KismetMathLibrary.BreakTransform` (`self.PreviousFloor`)))
  (bind _destination_location (`KismetMathLibrary.BreakTransform` (`self.Destination`)))
  (set `self.moves` true)
  (bind (_direction _shitass) (`Timeline|Move` :!via `PlayFromStart`)
    (:`Update`
      (`SceneComponent.K2_SetRelativeLocation` (`self.Beacon_ver_2_Lift_detail_1`) (`KismetMathLibrary.VLerp` _previousfloor_location _destination_location _shitass) true false))
    (:`Finished`
      (set `self.moves` false)
      (`self.I Am So Sorry`) ; what....?
      (`self.CheckIfPlayerDown`)
      ;[1 1 1] CameraShake
      (if (`self.isPlayerAboard?`)
        (`GameplayStatics.PlayWorldCameraShake` "/Game/FirstPerson/Blueprints/BP_CamShake.BP_CamShake_C" (`self.K2_GetActorLocation` (`self.Player`)) 0.0 1000.0)))))

(event `CheckIfPlayerDown`
  (if (== (`self.PreviousFloor`) (`SceneComponent.GetRelativeTransform` (`self.Floor 3`)))
    (if (< (.z (.location (`self.GetTransform` (`self.Player`)))) (`self.BeaconHeight`))
      (`self.Lift`))))

(fn `I Am So Sorry`
  (bind _output_get (set `self.PreviousFloor` (`self.Destination`)))
  (if (== _output_get (`SceneComponent.GetRelativeTransform` (`self.Floor 3`)))
    (set `self.goingUp?` false)
    (set `self.Destination` (`SceneComponent.GetRelativeTransform` (`self.Floor 2`)))
    (`KismetSystemLibrary.PrintString` "Floor2 Down")
    (elif (and (`self.goingUp?`) (== (`self.PreviousFloor`) (`SceneComponent.GetRelativeTransform` (`self.Floor 2`))))
      (set `self.Destination` (`SceneComponent.GetRelativeTransform` (`self.Floor 3`)))
      (`KismetSystemLibrary.PrintString` "Floor3")
      (elif (and (not (`self.goingUp?`)) (== (`self.PreviousFloor`) (`SceneComponent.GetRelativeTransform` (`self.Floor 2`))))
        (set `self.Destination` (`SceneComponent.GetRelativeTransform` (`self.Floor 1`)))
        (`KismetSystemLibrary.PrintString` "Floor1")
        (elif (== (`self.PreviousFloor`) (`SceneComponent.GetRelativeTransform` (`self.Floor 1`)))
          (set `self.goingUp?` true)
          (set `self.Destination` (`SceneComponent.GetRelativeTransform` (`self.Floor 2`)))
          (`KismetSystemLibrary.PrintString` "Floor2 Up"))))))

(fn `UserConstructionScript`)