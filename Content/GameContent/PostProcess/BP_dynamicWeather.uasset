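; Weather controller actor that applies a data asset preset to the level, setting the dawn preset on BeginPlay.
; UpdateWeather toggles Niagara rain and pushes preset values to the height fog, directional light and volumetric cloud actors, each found by class.
; Rain spawn rate and ocean steps are marked as not working, with the ocean wave setter left unwired.
; A timed loop cycling four time-of-day presets is also disconnected, so it never runs.
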(event `UpdateWeather`
  (bind _niagara (`self.Niagara`))
  (bind _data (`self.DATA`))
  (bind _data_2 (`self.DATA`))
  ;[1 1 1] Дождь
  (if (`/Game/GameContent/PostProcess/PDA_WeatherPresert.Rain` (`self.DATA`))
    (`SceneComponent.SetVisibility` (`self.Niagara`) true false)
    (else
      (`SceneComponent.SetVisibility` _niagara false false)))
  (`|ExecutionSequence`
    (:`then_0`
      (bind _returnvalue (`GameplayStatics.GetActorOfClass` "/Script/Engine.ExponentialHeightFog"))
      (`|ExecutionSequence`
        (:`then_0`
          (bind _component (`ExponentialHeightFog.Component` _returnvalue))
          (`ExponentialHeightFogComponent.SetVolumetricFogAlbedo` _component (`/Game/GameContent/PostProcess/PDA_WeatherPresert.FOG_Albedo` _data_2)))
        (:`then_1`
          (`ExponentialHeightFogComponent.SetVolumetricFogEmissive` _component (`/Game/GameContent/PostProcess/PDA_WeatherPresert.FOG_Emissive` _data_2)))
        (:`then_2`
          (`ExponentialHeightFogComponent.SetVolumetricFogExtinctionScale` _component (`/Game/GameContent/PostProcess/PDA_WeatherPresert.FOG_Extinction Scale` _data_2)))
        (:`then_3`
          (`ExponentialHeightFogComponent.SetStartDistance` _component (`/Game/GameContent/PostProcess/PDA_WeatherPresert.FOG_Start Distance` _data_2)))
        (:`then_4`
          (`ExponentialHeightFogComponent.SetFogDensity` _component (`/Game/GameContent/PostProcess/PDA_WeatherPresert.FOG_Density` _data_2)))
        (:`then_5`
          (`ExponentialHeightFogComponent.SetSecondFogDensity` _component (`/Game/GameContent/PostProcess/PDA_WeatherPresert.FOG_secondFogDensity` _data_2)))
        (:`then_6`
          (`ExponentialHeightFogComponent.SetFogHeightFalloff` _component (`/Game/GameContent/PostProcess/PDA_WeatherPresert.FOG_Height_Falloff` _data_2)))
        (:`then_7`
          (`ExponentialHeightFogComponent.SetSecondFogHeightFalloff` _component (`/Game/GameContent/PostProcess/PDA_WeatherPresert.FOG_first_height_falloff` _data_2)))
        (:`then_8`
          (`ExponentialHeightFogComponent.SetVolumetricFogScatteringDistribution` _component (`/Game/GameContent/PostProcess/PDA_WeatherPresert.FOG_scatteringDistribution` _data_2)))))
    (:`then_1`
      (bind _returnvalue_2 (`GameplayStatics.GetActorOfClass` "/Script/Engine.DirectionalLight"))
      (`|ExecutionSequence`
        (:`then_0`
          (bind _lightcomponent (`Light.LightComponent` _returnvalue_2))
          (`LightComponent.SetTemperature` _lightcomponent (`/Game/GameContent/PostProcess/PDA_WeatherPresert.DL_Temperature` _data)))
        (:`then_1`
          (`LightComponent.SetLightColor` _lightcomponent (`/Game/GameContent/PostProcess/PDA_WeatherPresert.DL_Light_Color` _data) true))))
    (:`then_2`
      ;[1 1 1] Не работает
      (`NiagaraComponent.SetVariableFloat` _niagara "SpawnRate" (`/Game/GameContent/PostProcess/PDA_WeatherPresert.RAIN_SpawnRate` (`self.DATA`))))
    (:`then_3`
      ;[1 1 1] Не работает
      (bind _returnvalue_3 (`GameplayStatics.GetActorOfClass` "/Script/Water.WaterBodyOcean")))
    (:`then_4`
      (bind _returnvalue_4 (`GameplayStatics.GetActorOfClass` "/Script/Engine.VolumetricCloud"))
      (`VolumetricCloudComponent.SetLayerBottomAltitude` (`VolumetricCloud.VolumetricCloudComponent` _returnvalue_4) (`/Game/GameContent/PostProcess/PDA_WeatherPresert.VolCloud_Layer_Bottom_Altitude` (`self.DATA`))))))

(event `self.ReceiveBeginPlay`
  (set `self.DATA` "/Game/GameContent/PostProcess/DA_Weather_2_dawn.DA_Weather_2_dawn")
  (`self.UpdateWeather`))

(event `self.ReceiveTick`
  (params (DeltaSeconds :type "Float (single-precision)")))

(fn `UserConstructionScript`)