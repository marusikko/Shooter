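; Barrel pickup actor that drifts toward a beacon and can be collected by the first-person character.
; Each tick it moves at Speed toward the Target_Beacon actor, looked up every frame, using a swept move.
; Box overlap by the character sets GotBarrel on player 0 and destroys the barrel, or prints a message if one is already held.
; Uncollected barrels destroy themselves after a fixed delay from BeginPlay.
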(event `self.ReceiveBeginPlay`
  (`KismetSystemLibrary.Delay` 50.0)
  (`self.K2_DestroyActor`))

(event `self.ReceiveTick`
  (params (DeltaSeconds :type "Float (single-precision)"))
  ;[1 1 1] Направление до маяка
  (bind _returnvalue (`GameplayStatics.GetActorOfClass` "/Game/GameContent/Enemy/AI_mark/Target_Beacon.Target_Beacon_C"))
  (`self.K2_SetActorLocation` (+ (* (`KismetMathLibrary.Normal` (- (`self.K2_GetActorLocation` _returnvalue) (`self.K2_GetActorLocation`))) (* (`GameplayStatics.GetWorldDeltaSeconds`) (`self.speed`))) (`self.K2_GetActorLocation`)) true))

(event `self.Box.OnComponentBeginOverlap`
  (params (OverlappedComponent :type "PrimitiveComponent Object Reference") (OtherActor :type "Actor Object Reference") (OtherComp :type "PrimitiveComponent Object Reference") (OtherBodyIndex :type Integer) (bFromSweep :type Boolean) (SweepResult :type "HitResult Structure (by ref)"))
  (bind _asbp_first_person_character (cast `/Game/FirstPerson/Blueprints/BP_FirstPersonCharacter` OtherActor))
  (if (`/Game/FirstPerson/Blueprints/BP_FirstPersonCharacter.GotBarrel` _asbp_first_person_character)
    (`KismetSystemLibrary.PrintString` "Already have barrel")
    (else
      (bind _asbp_first_person_character_2 (cast `/Game/FirstPerson/Blueprints/BP_FirstPersonCharacter` (`GameplayStatics.GetPlayerCharacter` 0)))
      (set `/Game/FirstPerson/Blueprints/BP_FirstPersonCharacter.GotBarrel` true _asbp_first_person_character_2)
      (`self.K2_DestroyActor`))))

(fn `UserConstructionScript`)