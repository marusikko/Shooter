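; Test zombie enemy character that takes two kinds of damage and dies when its HP runs out.
; TakeDamage removes 5 HP per 0.2-second Niagara burst, looping while its Damaging input is true, whereas TakeFlashDamage removes 1 HP per call.
; When HP drops below 1, either event halts walking, overrides the mesh animation with a dying clip and destroys the actor after a delay.
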(event `/Game/GameContent/Enemy/BPI_Damageable.TakeDamage`
  (params (Damaging :type Boolean))
  (`KismetSystemLibrary.PrintString` "DAMAGE!" true true (struct :`R` 1.0 :`G` 0.040124 :`A` 1.0) :!label _label)
  (`ActorComponent.Activate` (`self.Niagara`) false)
  (`KismetSystemLibrary.Delay` 0.2)
  (set `self.HP` (- (`self.HP`) 5))
  (`ActorComponent.Deactivate` (`self.Niagara`))
  (if (>= (`self.HP`) 1)
    (if Damaging
      (goto _label)
      (else
        (`KismetSystemLibrary.PrintString` "stop!")))
    (else
      (set `CharacterMovementComponent.MaxWalkSpeed` 0.0 (`self.CharacterMovement`))
      (`SkeletalMeshComponent.OverrideAnimationData` (`self.Mesh`) "/Game/GameContent/Enemy/AI_mark/Anim/Zombie_Dying.Zombie_Dying" false true 0.0 1.0)
      (`KismetSystemLibrary.Delay` 4.0)
      (`self.K2_DestroyActor`))))

(event `/Game/GameContent/Enemy/BPI_Damageable.TakeFlashDamage`
  (`KismetSystemLibrary.PrintString` "Flash Danmage" true true (struct :`R` 1.0 :`G` 0.857114 :`B` 0.169327 :`A` 1.0))
  (`ActorComponent.Activate` (`self.Niagara`) false)
  (`KismetSystemLibrary.Delay` 0.2)
  (set `self.HP` (- (`self.HP`) 1))
  (`ActorComponent.Deactivate` (`self.Niagara`))
  (if (not (>= (`self.HP`) 1))
    (set `CharacterMovementComponent.MaxWalkSpeed` 0.0 (`self.CharacterMovement`))
    (`SkeletalMeshComponent.OverrideAnimationData` (`self.Mesh`) "/Game/GameContent/Enemy/AI_mark/Anim/Zombie_Dying.Zombie_Dying" false true 0.0 1.0)
    (`KismetSystemLibrary.Delay` 4.0)
    (`self.K2_DestroyActor`)))

(fn `UserConstructionScript`)