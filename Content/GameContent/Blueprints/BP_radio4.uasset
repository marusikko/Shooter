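; BP_radio4 is a one-shot radio trigger that plays audio and blinks a light when the player character enters its Box.
; The overlap plays RadioBeep, then after a short delay plays Water_4, both attenuated at the actor's location, and sets Played.
; A counted Delay loop then toggles the PointLight's intensity for 21 blinks, leaving it off.
; Played is set only after the first delay, so re-entering during it replays the beep.
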(event `self.Box.OnComponentBeginOverlap`
  (params (OverlappedComponent :type "PrimitiveComponent Object Reference") (OtherActor :type "Actor Object Reference") (OtherComp :type "PrimitiveComponent Object Reference") (OtherBodyIndex :type Integer) (bFromSweep :type Boolean) (SweepResult :type "HitResult Structure (by ref)"))
  (bind _returnvalue (`self.K2_GetActorLocation`))
  (if (== OtherActor (`GameplayStatics.GetPlayerCharacter` 0))
    (if (not (`self.Played`))
      (`GameplayStatics.PlaySoundAtLocation` "/Game/GameContent/Sounds/Radio/RadioBeep.RadioBeep" _returnvalue (struct) 1.0 1.0 0.0 "/Game/GameContent/Sounds/SoundAttenuation.SoundAttenuation" null null null)
      (`KismetSystemLibrary.Delay` 0.5)
      (`GameplayStatics.PlaySoundAtLocation` "/Game/GameContent/Sounds/Radio/Water_4.Water_4" _returnvalue (struct) 1.0 1.0 0.0 "/Game/GameContent/Sounds/SoundAttenuation.SoundAttenuation" null null null)
      (set `self.Played` true)
      (`LightComponent.SetIntensity` (`self.PointLight`) 0.0 :!label _label)
      (`KismetSystemLibrary.Delay` 0.5)
      (`LightComponent.SetIntensity` (`self.PointLight`) 2000.0)
      (`KismetSystemLibrary.Delay` 0.5)
      (`LightComponent.SetIntensity` (`self.PointLight`) 0.0)
      (set `self.LightBeeps` (+ (`self.LightBeeps`) 1))
      (if (not (>= (`self.LightBeeps`) 21))
        (goto _label)))))

(fn `UserConstructionScript`)