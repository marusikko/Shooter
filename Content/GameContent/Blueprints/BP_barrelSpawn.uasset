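; BP_barrelSpawn is a spawner that repeatedly creates BP_barrel actors around a set of stored Locations once the tutorial is finished.
; From BeginPlay it polls the TutorialFin flag on a short delay, then enters an endless timed loop that spawns one barrel per location.
; Each spawn gets a random positive X and Y offset from its transform, adjusting for collisions but always spawning.
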(event `self.ReceiveBeginPlay`
  (`KismetSystemLibrary.Delay` 1.0 :!label _label)
  (if (`self.TutorialFin`)
    (for _array_element (`self.locations`) :!label _label_2
      (`|SpawnActorFromClass` "/Game/GameContent/meshes/BP_barrel.BP_barrel_C" (`KismetMathLibrary.MakeTransform` (`KismetMathLibrary.MakeVector` (+ (.x (.location _array_element)) (`KismetMathLibrary.RandomInteger` 4000)) (+ (.y (.location _array_element)) (`KismetMathLibrary.RandomInteger` 4000)) (.z (.location _array_element))) (.rotation _array_element) (.scale _array_element)) "AdjustIfPossibleButAlwaysSpawn" "MultiplyWithRoot" null null))
    (`KismetSystemLibrary.Delay` 10.0)
    (goto _label_2)
    (else
      (goto _label))))

(fn `UserConstructionScript`)