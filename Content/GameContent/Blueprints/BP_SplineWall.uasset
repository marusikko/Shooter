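; Spline-driven wall builder that tiles a chosen static mesh along a spline in the Construction Script.
; Segment count comes from spline length divided by the mesh's bounding-box size on the alignment axis, with at least one segment.
; Each spline mesh takes position, tangents and roll from the spline, with OffsetControl scaling end distances and RollControl adding roll.
; Start and end scales are randomised independently from a random stream within set limits, multiplied by ScaleControl.
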(fn `UserConstructionScript`
  (bind _random_stream (`self.Random Stream`))
  (bind _max_scale_randomness (`self.Max Scale Randomness`))
  (bind _min_scale_randomness (`self.Min Scale Randomness`))
  (bind _spline (`self.Spline`))
  (bind _spline_2 (`self.Spline`))
  (bind (_returnvalue_min _returnvalue_max) (break `Box` (`StaticMesh.GetBoundingBox` (`self.Mesh to Spawn`))))
  (bind _returnvalue (`KismetMathLibrary.DegreesToRadians` (`self.Roll Control`)))
  (bind (_returnvalue_x _returnvalue_y _returnvalue_z) (`KismetMathLibrary.BreakVector` (- _returnvalue_max _returnvalue_min)))
  (bind _returnvalue_2 (* (`self.Scale Control`) (`KismetMathLibrary.MakeVector2D` (`KismetMathLibrary.RandomFloatInRangeFromStream` _random_stream _min_scale_randomness _max_scale_randomness) (`KismetMathLibrary.RandomFloatInRangeFromStream` _random_stream _min_scale_randomness _max_scale_randomness))))
  (bind _returnvalue_3 (`KismetMathLibrary.Abs` (select `ESplineMeshAxis` (`self.Mesh Alignment Axis`) :`X` _returnvalue_x :`Y` _returnvalue_y :`Z` _returnvalue_z)))
  (`self.Mesh to Spawn`
    (:`then`
      ;[1 1 1] Loop and set mesh
      (for _index (range (+ (`KismetMathLibrary.Max` (- (`KismetMathLibrary.FFloor` (/ (`SplineComponent.GetSplineLength` (`self.Spline`)) _returnvalue_3)) 1)) 1))
        (bind _returnvalue_4 (`AddComponent|NODE_AddSplineMeshComponent-0`))
        (`StaticMeshComponent.SetStaticMesh` _returnvalue_4 (`self.Mesh To Spawn`))
        (bind _returnvalue_5 (* _index _returnvalue_3))
        (bind _returnvalue_6 (* (* (+ _index 1) _returnvalue_3) (`self.Offset Control`)))
        ;[1 1 1] Work through the spline for additional transforms
        (`SplineMeshComponent.SetStartAndEnd` _returnvalue_4 (`SplineComponent.GetLocationAtDistanceAlongSpline` _spline_2 _returnvalue_5 "Local") (* (`SplineComponent.GetDirectionAtDistanceAlongSpline` _spline_2 _returnvalue_5 "Local") _returnvalue_3) (`SplineComponent.GetLocationAtDistanceAlongSpline` _spline _returnvalue_6 "Local") (* (`SplineComponent.GetDirectionAtDistanceAlongSpline` _spline _returnvalue_6 "Local") _returnvalue_3) true)
        (`SplineMeshComponent.SetEndScale` _returnvalue_4 _returnvalue_2 true)
        (`SplineMeshComponent.SetStartScale` _returnvalue_4 _returnvalue_2 true)
        (`SplineMeshComponent.SetForwardAxis` _returnvalue_4 (`self.Mesh Alignment Axis`) true)
        ;[1 1 1] Roll
        (`SplineMeshComponent.SetStartRoll` _returnvalue_4 (+ (`KismetMathLibrary.DegreesToRadians` (`SplineComponent.GetRollAtDistanceAlongSpline` _spline _returnvalue_5 "Local")) _returnvalue) true)
        (`SplineMeshComponent.SetEndRoll` _returnvalue_4 (+ (`KismetMathLibrary.DegreesToRadians` (`SplineComponent.GetRollAtDistanceAlongSpline` _spline _returnvalue_6 "Local")) _returnvalue) true)))
    (:`else`)))